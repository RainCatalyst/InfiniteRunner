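; RunnerGamemode is the game mode for a runner game, owning player health and the game-over flow.
; It creates a full HealthBar widget on BeginPlay.
; Damage applied to the game mode itself through AnyDamage is truncated to an integer, subtracted from clamped health and reflected in the bar.
; At zero health, GameOver adds the GameOverMenu widget, shows the mouse cursor and pauses the game.
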(event EventBeginPlay
  (bind _returnvalue (UserInterface|CreateWidget "/Game/Blueprints/HealthBar.HealthBar_C"))
  (UserInterface|Viewport|AddtoViewport _returnvalue 0)
  (bind _output_get (Variables|Default|SetHealthBar _returnvalue))
  (Default|SetPercent _output_get 1.0))

(event EventTick
  (params (DeltaSeconds :type Float%20%28single-precision%29)))

(event Game|Damage|EventAnyDamage
  (params (Damage :type Float%20%28single-precision%29) (DamageType :type Damage%20Type%20Object%20Reference) (InstigatedBy :type Controller%20Object%20Reference) (DamageCauser :type Actor%20Object%20Reference))
  (CallFunction|OnDamageTaken (Math|Float|Truncate Damage)))

(fn ConstructionScript)

(fn OnDamageTaken
  (params (Damage :type Integer))
  (bind _output_get (Variables|Default|SetCurrentHealth (Math|Integer|Clamp(Integer) (- (Variables|Default|GetCurrentHealth) Damage) 0 (Variables|Default|GetMaxHealth))))
  (Default|SetPercent (Variables|Default|GetHealthBar) (/ (Math|Conversions|ToFloat(Integer) _output_get) (Variables|Default|GetMaxHealth)))
  (Math|Integer|CompareInt _output_get
    (:==
      (Development|PrintString "Game Over!!!")
      (CallFunction|GameOver))))

(fn GameOver
  (bind _returnvalue (UserInterface|CreateWidget "/Game/Blueprints/GameOverMenu.GameOverMenu_C"))
  (UserInterface|Viewport|AddtoViewport _returnvalue 0)
  (Variables|/Script/Engine.PlayerController|SetbShowMouseCursor (Game|GetPlayerController 0) true)
  (Game|SetGamePaused true))